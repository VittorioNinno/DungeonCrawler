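; BP_EnemyBase is an enemy Blueprint that wanders at random and moves toward a target.
; From BeginPlay it moves to a random navigable point around itself, waits after success or failure, then repeats only while CurrentTarget is invalid.
; Tick issues AIMoveTo toward CurrentTarget every frame while EnemyState is 1.
; These graphs only read the state and target, and never set them.
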(event Custom|RandomMovement
  (bind _randomlocation (Class|NavigationSystemV1|GetRandomLocationinNavigableRadius (Transformation|GetActorLocation) 5e+02 0 0))
  (AI|AIMoveTo self _randomlocation 0 5.0 false
    (:OnSuccess
      _)
    (:OnFail
      _))
  (Utilities|FlowControl|Delay (Variables|Default|GetWaitTimeAfterMovement))
  (if (not (Utilities|IsValid (Variables|Default|GetCurrentTarget)))
    (CallFunction|RandomMovement)))

(event EventBeginPlay
  (CallFunction|RandomMovement))

(event EventTick
  (params (DeltaSeconds :type Float%20%28single-precision%29))
  (if (== (Variables|Default|GetEnemyState) 1)
    (AI|AIMoveTo self "0, 0, 0" (Variables|Default|GetCurrentTarget) 5.0 false)))

(fn ConstructionScript)